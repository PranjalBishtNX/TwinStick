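; Rail prop Blueprint that assembles a line of rail pieces from instanced meshes in its construction script.
; It places a scaled, rotated RailEnd, then repeats Rail at fixed spacing along X up to a variable count.
; A raised RailMount follows at the last loop index, and a second variable-length run of Rail continues from the accumulated count.
; The event graph contains only disabled stub events.
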(event EventBeginPlay)

(event Collision|EventActorBeginOverlap
  (params (OtherActor :type Actor%20Object%20Reference)))

(event EventTick
  (params (DeltaSeconds :type Float%20%28single-precision%29)))

(fn ConstructionScript
  (Components|InstancedStaticMesh|AddInstance (Variables|Default|GetRail_End) (Math|Transform|MakeTransform "200.000000, 0, 0" "90.000000, 0, 0" "1.500000,1.500000,1.500000"))
  (for _index (range 1 (Variables|Default|GetINT))
    (Components|InstancedStaticMesh|AddInstance (Variables|Default|GetRail) (Math|Transform|MakeTransform (Math|Vector|MakeVector (* _index 1e+03) 0.0 0.0) "0, 0, 0" "1,1,1"))
    (Variables|Default|SetRailCOunt (+ (Variables|Default|GetRailCOunt) 1.0)))
  (Components|InstancedStaticMesh|AddInstance (Variables|Default|GetRail_Mount) (Math|Transform|MakeTransform (Math|Vector|MakeVector (* _index 1e+03) 0.0 5e+01) "0, 0, 0" "1,1,1"))
  (for _index_2 (range 0 (Variables|Default|GetINT_01))
    (Components|InstancedStaticMesh|AddInstance (Variables|Default|GetRail) (Math|Transform|MakeTransform (Math|Vector|MakeVector (* (+ (Math|Conversions|ToFloat(Integer) _index_2) (Variables|Default|GetRailCOunt)) 1e+03) 0.0 0.0) "0, 0, 0" "1,1,1"))))