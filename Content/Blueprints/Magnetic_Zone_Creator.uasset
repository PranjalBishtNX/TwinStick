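; Magnetic zone helper that detects when the player ball enters the magnetic field of its closest wall.
; Each Tick, while a magnetic wall is close by, it sphere-overlaps at the wall collision point nearest the ball and writes the in-zone flag back to the player.
; During wall ride, it also aims the player's WallPointer at that point.
; The zone is drawn as a debug sphere; the Sphere-moving node is unwired.
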(event EventBeginPlay)

(event Collision|EventActorBeginOverlap
  (params (OtherActor :type Actor%20Object%20Reference)))

(event EventTick
  (params (DeltaSeconds :type Float%20%28single-precision%29))
  (Utilities|FlowControl|Sequence
    (:then_0
      (bind _asplayer_ball_bp (Utilities|Casting|CastToPlayer_Ball_Bp (Pawn|GetControlledPawn (Class|GameplayStatics|GetPlayerControllerfromID))))
      (bind _asmagnetic_walls_1_1 (Utilities|Casting|CastToMagnetic_Walls_1_1 (Variables|/Game/Blueprints/Player_Ball_Bp.Player_Ball_Bp_C|GetClosest%20Wall _asplayer_ball_bp)))
      (if (Variables|/Game/Blueprints/Player_Ball_Bp.Player_Ball_Bp_C|GetMagnetic%20Wall%20is%20close%20by _asplayer_ball_bp)
        (bind _returnvalue (Collision|SphereOverlapActors (.OutPointOnBody (Collision|GetClosestPointonCollision (Variables|/Game/Blueprints/Magnetic_Walls_1_1.Magnetic_Walls_1_1_C|GetWallDefault _asmagnetic_walls_1_1) (Transformation|GetWorldLocation (Variables|/Game/Blueprints/Player_Ball_Bp.Player_Ball_Bp_C|GetMovingSphere _asplayer_ball_bp)) "None")) 2e+02 (Utilities|Array|MakeArray "ObjectTypeQuery4") "/Game/Blueprints/Player_Ball_Bp.Player_Ball_Bp_C"))
        (Rendering|Debug|DrawDebugSphere (.OutPointOnBody (Collision|GetClosestPointonCollision (Variables|/Game/Blueprints/Magnetic_Walls_1_1.Magnetic_Walls_1_1_C|GetWallDefault _asmagnetic_walls_1_1) (Transformation|GetWorldLocation (Variables|/Game/Blueprints/Player_Ball_Bp.Player_Ball_Bp_C|GetMovingSphere _asplayer_ball_bp)) "None")) 2e+02 12 "(R=1.000000,G=0.219716,B=0.000000,A=1.000000)" 0.0 2.0)
        (Variables|/Game/Blueprints/Player_Ball_Bp.Player_Ball_Bp_C|SetVehicle%20Is%20inside%20Magnetic%20Wall%20zone _asplayer_ball_bp _returnvalue)))
    (:then_1
      (if (Variables|/Game/Blueprints/Player_Ball_Bp.Player_Ball_Bp_C|GetWallRideActivate _asplayer_ball_bp)
        (Transformation|SetWorldRotation (Variables|/Game/Blueprints/Player_Ball_Bp.Player_Ball_Bp_C|GetWallPointer _asplayer_ball_bp) (Math|Rotator|FindLookatRotation (Transformation|GetWorldLocation (Variables|/Game/Blueprints/Player_Ball_Bp.Player_Ball_Bp_C|GetMovingSphere _asplayer_ball_bp)) (.OutPointOnBody (Collision|GetClosestPointonCollision (Variables|/Game/Blueprints/Magnetic_Walls_1_1.Magnetic_Walls_1_1_C|GetWallDefault _asmagnetic_walls_1_1) (Transformation|GetWorldLocation (Variables|/Game/Blueprints/Player_Ball_Bp.Player_Ball_Bp_C|GetMovingSphere _asplayer_ball_bp)) "None"))) false false)))))

(fn ConstructionScript)