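; Energy barrier prop that builds a configurable rectangular box of barrier walls entirely in its construction script, with no active runtime logic.
; Nested loops over Height, Length and Width tile static mesh panels on a 1000-unit grid along all four sides, rotating the widthwise ones 90 degrees.
; A second pass lays glow meshes around the bottom perimeter.
; ColVariation 1 swaps panels and glow to red materials.
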(event EventBeginPlay)

(event Collision|EventActorBeginOverlap
  (params (OtherActor :type Actor%20Object%20Reference)))

(event EventTick
  (params (DeltaSeconds :type Float%20%28single-precision%29)))

(fn ConstructionScript
  ;[1 1 1] Main Loop, runs for each height unit
  (for _index (range 0 (- (Variables|Default|GetHeight) 1))
    (for _index_2 (range 0 (- (Variables|Default|GetLength) 1))
      ;[1 1 1] Lengthwise Side 1
      (bind _returnvalue (AddComponent|AddStaticMeshComponent false (Math|Conversions|ToTransform(Vector) (+ (* "0, 0,1000.000000" _index) (* "1000.000000, 0,0.000000" _index_2)))))
      (if (== (Variables|Default|GetCol_Variation) 1)
        (Rendering|Material|SetMaterial _returnvalue 0 "/Game/Materials/GenericTiled/Mat_SF_Barrier_Red.Mat_SF_Barrier_Red"))
      ;[1 1 1] Lengthwise Side 2
      (bind _returnvalue_2 (AddComponent|AddStaticMeshComponent false (Math|Conversions|ToTransform(Vector) (+ (* "0.000000,1000.000000,0.000000" (Variables|Default|GetWidth)) (+ (* "0, 0,1000.000000" _index) (* "1000.000000, 0,0.000000" _index_2))))))
      (if (== (Variables|Default|GetCol_Variation) 1)
        (Rendering|Material|SetMaterial _returnvalue_2 0 "/Game/Materials/GenericTiled/Mat_SF_Barrier_Red.Mat_SF_Barrier_Red")))
    (for _index_3 (range 0 (- (Variables|Default|GetWidth) 1))
      ;[1 1 1] Widthwise Side 1
      (bind _returnvalue_3 (AddComponent|AddStaticMeshComponent false (Math|Conversions|ToTransform(Vector) (+ (* "0.000000,1000.000000,0.000000" _index_3) (* "0, 0,1000.000000" _index)))))
      (Transformation|AddLocalRotation _returnvalue_3 "0.000000,90.000000,0.000000" false false)
      (if (== (Variables|Default|GetCol_Variation) 1)
        (Rendering|Material|SetMaterial _returnvalue_3 0 "/Game/Materials/GenericTiled/Mat_SF_Barrier_Red.Mat_SF_Barrier_Red"))
      ;[1 1 1] Widthwise Side 2
      (bind _returnvalue_4 (AddComponent|AddStaticMeshComponent false (Math|Conversions|ToTransform(Vector) (+ (* "1000.000000,0.000000,0.000000" (Variables|Default|GetLength)) (+ (* "0.000000,1000.000000,0.000000" _index_3) (* "0, 0,1000.000000" _index))))))
      (Transformation|AddLocalRotation _returnvalue_4 "0.000000,90.000000,0.000000" false false)
      (if (== (Variables|Default|GetCol_Variation) 1)
        (Rendering|Material|SetMaterial _returnvalue_4 0 "/Game/Materials/GenericTiled/Mat_SF_Barrier_Red.Mat_SF_Barrier_Red"))))
  ;[1 1 1] Bottom Glow mesh
  (for _index_4 (range 0 (- (Variables|Default|GetLength) 1))
    (bind _returnvalue_5 (AddComponent|AddStaticMeshComponent false (Math|Conversions|ToTransform(Vector) (* "1000.000000, 0,0.000000" _index_4))))
    (if (== (Variables|Default|GetCol_Variation) 1)
      (Rendering|Material|SetMaterial _returnvalue_5 0 "/Game/Materials/GenericTiled/Mat_SF_Barrier_Bottom_Red.Mat_SF_Barrier_Bottom_Red"))
    (bind _returnvalue_6 (AddComponent|AddStaticMeshComponent false (Math|Conversions|ToTransform(Vector) (+ (* "0.000000,1000.000000,0.000000" (Variables|Default|GetWidth)) (* "1000.000000, 0,0.000000" _index_4)))))
    (if (== (Variables|Default|GetCol_Variation) 1)
      (Rendering|Material|SetMaterial _returnvalue_6 0 "/Game/Materials/GenericTiled/Mat_SF_Barrier_Bottom_Red.Mat_SF_Barrier_Bottom_Red")))
  ;[1 1 1] Bottom Glow mesh widthwise
  (for _index_5 (range 0 (- (Variables|Default|GetWidth) 1))
    (bind _returnvalue_7 (AddComponent|AddStaticMeshComponent false (Math|Conversions|ToTransform(Vector) (* "0.000000,1000.000000,0.000000" _index_5))))
    (Transformation|AddLocalRotation _returnvalue_7 "0.000000,90.000000,0.000000" false false)
    (if (== (Variables|Default|GetCol_Variation) 1)
      (Rendering|Material|SetMaterial _returnvalue_7 0 "/Game/Materials/GenericTiled/Mat_SF_Barrier_Bottom_Red.Mat_SF_Barrier_Bottom_Red"))
    (bind _returnvalue_8 (AddComponent|AddStaticMeshComponent false (Math|Conversions|ToTransform(Vector) (+ (* "1000.000000,0.000000,0.000000" (Variables|Default|GetLength)) (* "0.000000,1000.000000,0.000000" _index_5)))))
    (Transformation|AddLocalRotation _returnvalue_8 "0.000000,90.000000,0.000000" false false)
    (if (== (Variables|Default|GetCol_Variation) 1)
      (Rendering|Material|SetMaterial _returnvalue_8 0 "/Game/Materials/GenericTiled/Mat_SF_Barrier_Bottom_Red.Mat_SF_Barrier_Bottom_Red"))))