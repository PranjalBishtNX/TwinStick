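; Spline-driven track prop that lays a chosen track mesh along an editable spline.
; The construction script adds a spline mesh segment at each spacing step, with a thickness scale multiplying cross-section, spacing and tangent length.
; Each segment takes world-space position, direction and roll from the spline at both ends, using manual attachment.
; The event graph has no active logic.
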(event EventBeginPlay)

(event Collision|EventActorBeginOverlap
  (params (OtherActor :type Actor%20Object%20Reference)))

(event EventTick
  (params (DeltaSeconds :type Float%20%28single-precision%29)))

(fn ConstructionScript
  (bind _returnvalue (Class|KismetMathLibrary|Vector2DOne))
  (bind _thickless_scale (Variables|Default|GetThickless_Scale))
  (bind _spline (Variables|Default|GetSpline))
  (bind _spline_2 (Variables|Default|GetSpline))
  (bind _curvature (Variables|Default|GetCurvature))
  (bind _thickless_scale_2 (Variables|Default|GetThickless_Scale))
  (bind _thickless_scale_3 (Variables|Default|GetThickless_Scale))
  (bind _spacing (Variables|Default|GetSpacing))
  (bind _returnvalue_2 (* _returnvalue _thickless_scale))
  (bind _returnvalue_3 (* _spacing _thickless_scale_2))
  (bind _returnvalue_4 (* _curvature _thickless_scale_3))
  (for _index (range 0 (Math|Integer|Max(Integer) (- (.ReturnValue (Math|Float|Division(WholeandRemainder) (Spline|GetSplineLength _spline) _returnvalue_3)) 1)))
    (bind _returnvalue_5 (AddComponent|AddSplineMeshComponent true))
    (Components|StaticMesh|SetStaticMesh _returnvalue_5 (Variables|Default|GetTrackMesh))
    (SplineMesh|SetStartScale _returnvalue_5 _returnvalue_2 true :!class /Script/Engine.SplineMeshComponent)
    (SplineMesh|SetEndScale _returnvalue_5 _returnvalue_2 true :!class /Script/Engine.SplineMeshComponent)
    (SplineMesh|SetStartandEnd _returnvalue_5 (Spline|GetLocationatDistanceAlongSpline _spline (* (Math|Conversions|ToFloat(Integer) _index) _returnvalue_3) "World") (* (Spline|GetDirectionatDistanceAlongSpline _spline (* (Math|Conversions|ToFloat(Integer) _index) _returnvalue_3) "World") _returnvalue_4) (Spline|GetLocationatDistanceAlongSpline _spline (+ (* (Math|Conversions|ToFloat(Integer) _index) _returnvalue_3) _returnvalue_3) "World") (* (Spline|GetDirectionatDistanceAlongSpline _spline (+ (* (Math|Conversions|ToFloat(Integer) _index) _returnvalue_3) _returnvalue_3) "World") _returnvalue_4) true :!class /Script/Engine.SplineMeshComponent)
    (Class|SplineMeshComponent|SetStartRoll _returnvalue_5 (Math|Trig|DegreesToRadians (.Roll (Math|Rotator|BreakRotator (Spline|GetRotationatDistanceAlongSpline _spline_2 (* (Math|Conversions|ToFloat(Integer) _index) _returnvalue_3) "World")))) true)
    (Class|SplineMeshComponent|SetEndRoll _returnvalue_5 (Math|Trig|DegreesToRadians (.Roll (Math|Rotator|BreakRotator (Spline|GetRotationatDistanceAlongSpline _spline_2 (+ (* (Math|Conversions|ToFloat(Integer) _index) _returnvalue_3) _returnvalue_3) "World")))) true)))