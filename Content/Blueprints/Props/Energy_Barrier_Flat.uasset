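; Energy barrier prop that builds a flat wall of static mesh panels in its construction script, with no active runtime logic.
; Nested loops tile panels 1000 units apart along X for Length and up Z for Height.
; An optional BottomGlowOn pass adds a row of glow meshes along the base.
; ColVariation 1 swaps both panel and glow materials to red versions.
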(event EventBeginPlay)

(event Collision|EventActorBeginOverlap
  (params (OtherActor :type Actor%20Object%20Reference)))

(event EventTick
  (params (DeltaSeconds :type Float%20%28single-precision%29)))

(fn ConstructionScript
  (for _index (range 0 (- (Variables|Default|GetHeight) 1))
    (for _index_2 (range 0 (- (Variables|Default|GetLength) 1))
      (bind _returnvalue (AddComponent|AddStaticMeshComponent false (Math|Conversions|ToTransform(Vector) (+ (* "0, 0,1000.000000" _index) (* "1000.000000, 0,0.000000" _index_2)))))
      (if (== (Variables|Default|GetCol_Variation) 1)
        (Rendering|Material|SetMaterial _returnvalue 0 "/Game/Materials/GenericTiled/Mat_SF_Barrier_Red.Mat_SF_Barrier_Red"))))
  (if (Variables|Default|GetBottom%20Glow%20On)
    (for _index_3 (range 0 (- (Variables|Default|GetLength) 1))
      (bind _returnvalue_2 (AddComponent|AddStaticMeshComponent false (Math|Conversions|ToTransform(Vector) (* "1000.000000, 0,0.000000" _index_3))))
      (if (== (Variables|Default|GetCol_Variation) 1)
        (Rendering|Material|SetMaterial _returnvalue_2 0 "/Game/Materials/GenericTiled/Mat_SF_Barrier_Bottom_Red.Mat_SF_Barrier_Bottom_Red")))))