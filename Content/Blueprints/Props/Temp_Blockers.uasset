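; Temporary blocker prop that only appears while the ball player is in a challenge.
; On BeginPlay its Cube mesh is hidden with collision disabled.
; Every Tick it casts the player pawn to Player_Ball_Bp and reads ChallengeActiveStatus, showing the cube with query and physics collision when true and hiding it without collision otherwise.
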(event EventBeginPlay
  (Rendering|SetVisibility (Variables|Default|GetCube) false false)
  (Collision|SetCollisionEnabled (Variables|Default|GetCube) "NoCollision"))

(event Collision|EventActorBeginOverlap
  (params (OtherActor :type Actor%20Object%20Reference)))

(event EventTick
  (params (DeltaSeconds :type Float%20%28single-precision%29))
  (bind _asplayer_ball_bp (Utilities|Casting|CastToPlayer_Ball_Bp (Game|Player|GetPlayerPawn 0)))
  (if (Variables|/Game/Blueprints/Player/Player_Ball_Bp.Player_Ball_Bp_C|GetChallenge%20Active%20Status _asplayer_ball_bp)
    (Rendering|SetVisibility (Variables|Default|GetCube) true false)
    (Collision|SetCollisionEnabled (Variables|Default|GetCube) "QueryAndPhysics")
    (else
      (Rendering|SetVisibility (Variables|Default|GetCube) false false)
      (Collision|SetCollisionEnabled (Variables|Default|GetCube) "NoCollision"))))

(fn ConstructionScript)