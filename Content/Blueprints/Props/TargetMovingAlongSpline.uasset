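; Rail-riding actor that carries the player ball along its closest spline.
; Each tick, the rail component shadows the ball along the spline until the rail sphere trigger is entered.
; It then advances at a fixed per-tick step, pulling the ball to the matched find sphere and blending to the rail camera.
; A dot product picks travel direction and spring arm facing, while A/D roll the rail.
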(event Custom|Attatch%20Player%20Character%20to%20the%20rail%20sphere
  (bind _returnvalue (Utilities|Time|GetWorldDeltaSeconds))
  ;[1 1 1] Remake
  ;;[1 1 1] Attatching the player vehicle to the rail
  (if (Variables|/Game/Blueprints/Player/Player_Ball_Bp.Player_Ball_Bp_C|GetVehicle%20has%20entered%20Rail%20sphere%20Trigger (stale EventTick _asplayer_ball_bp))
    (Physics|SetPhysicsLinearVelocity (Variables|/Game/Blueprints/Player/Player_Ball_Bp.Player_Ball_Bp_C|GetMovingSphere (stale EventTick _asplayer_ball_bp)) "0, 0, 0" false "None")
    (Transformation|SetWorldLocationAndRotation (Variables|/Game/Blueprints/Player/Player_Ball_Bp.Player_Ball_Bp_C|GetMovingSphere (stale EventTick _asplayer_ball_bp)) (Math|Interpolation|VInterpTo (Transformation|GetWorldLocation (Variables|/Game/Blueprints/Player/Player_Ball_Bp.Player_Ball_Bp_C|GetMovingSphere (stale EventTick _asplayer_ball_bp))) (Transformation|GetWorldLocation (Variables|Default|GetScene%20Component%20Object%20reference)) (Utilities|Time|GetWorldDeltaSeconds) 2e+01) "0, 0, 0" false false)
    (bind _output_get (Variables|Default|SetLast%20Known%20Rail%20Location (Math|Float|Clamp(Float) (+ (Variables|Default|GetLast%20Known%20Rail%20Location) (* 4e+01 (Variables|Default|GetFacing%20Right%20Multiplier))) 0.0 (Spline|GetSplineLength (Actor|GetComponentbyClass (Variables|/Game/Blueprints/Player/Player_Ball_Bp.Player_Ball_Bp_C|GetClosestSpline (stale EventTick _asplayer_ball_bp)) "/Script/Engine.SplineComponent")))))
    (Transformation|SetWorldLocation (Variables|Default|GetRail%20Actor) (Spline|GetLocationatDistanceAlongSpline (Actor|GetComponentbyClass (Variables|/Game/Blueprints/Player/Player_Ball_Bp.Player_Ball_Bp_C|GetClosestSpline (stale EventTick _asplayer_ball_bp)) "/Script/Engine.SplineComponent") _output_get "World") false false)
    (Transformation|SetWorldRotation (Variables|Default|GetRail%20Actor) (Math|Rotator|MakeRotator (+ (.roll (Spline|GetRotationatDistanceAlongSpline (Actor|GetComponentbyClass (Variables|/Game/Blueprints/Player/Player_Ball_Bp.Player_Ball_Bp_C|GetClosestSpline (stale EventTick _asplayer_ball_bp)) "/Script/Engine.SplineComponent") _output_get "World")) (Variables|Default|GetRotational)) (.pitch (Spline|GetRotationatDistanceAlongSpline (Actor|GetComponentbyClass (Variables|/Game/Blueprints/Player/Player_Ball_Bp.Player_Ball_Bp_C|GetClosestSpline (stale EventTick _asplayer_ball_bp)) "/Script/Engine.SplineComponent") _output_get "World")) (.yaw (Spline|GetRotationatDistanceAlongSpline (Actor|GetComponentbyClass (Variables|/Game/Blueprints/Player/Player_Ball_Bp.Player_Ball_Bp_C|GetClosestSpline (stale EventTick _asplayer_ball_bp)) "/Script/Engine.SplineComponent") _output_get "World"))) false false)
    (Transformation|SetWorldLocationAndRotation (Variables|/Game/Blueprints/Player/Player_Ball_Bp.Player_Ball_Bp_C|GetCamera (stale EventTick _asplayer_ball_bp)) (Math|Interpolation|VInterpTo (Transformation|GetWorldLocation (Variables|/Game/Blueprints/Player/Player_Ball_Bp.Player_Ball_Bp_C|GetCamera (stale EventTick _asplayer_ball_bp))) (Transformation|GetWorldLocation (Variables|Default|GetRail%20Camera)) _returnvalue 2e+01) (Math|Interpolation|RInterpTo (Transformation|GetWorldRotation (Variables|/Game/Blueprints/Player/Player_Ball_Bp.Player_Ball_Bp_C|GetCamera (stale EventTick _asplayer_ball_bp))) (Transformation|GetWorldRotation (Variables|Default|GetRail%20Camera)) _returnvalue 2e+01) false false)))

(event Custom|Set%20the%20found%20closest%20rail%20sphere
  (bind _sphere_find_01 (Variables|Default|GetSphere_Find_01))
  (bind _sphere_find_02 (Variables|Default|GetSphere_Find_02))
  (bind _sphere_find_03 (Variables|Default|GetSphere_Find_03))
  (bind _sphere_find_04 (Variables|Default|GetSphere_Find_04))
  (Utilities|FlowControl|Sequence
    (:then_0
      ;[1 1 1] Sphere_Find_01
      (if (== _sphere_find_01 (Variables|/Game/Blueprints/Player/Player_Ball_Bp.Player_Ball_Bp_C|GetClosest%20rail%20Sphere (stale EventTick _asplayer_ball_bp)))
        (Variables|Default|SetScene%20Component%20Object%20reference _sphere_find_01)))
    (:then_1
      ;[1 1 1] Sphere_Find_02
      (if (== _sphere_find_02 (Variables|/Game/Blueprints/Player/Player_Ball_Bp.Player_Ball_Bp_C|GetClosest%20rail%20Sphere (stale EventTick _asplayer_ball_bp)))
        (Variables|Default|SetScene%20Component%20Object%20reference _sphere_find_02)))
    (:then_2
      ;[1 1 1] Sphere_Find_03
      (if (== _sphere_find_03 (Variables|/Game/Blueprints/Player/Player_Ball_Bp.Player_Ball_Bp_C|GetClosest%20rail%20Sphere (stale EventTick _asplayer_ball_bp)))
        (Variables|Default|SetScene%20Component%20Object%20reference _sphere_find_03)))
    (:then_3
      ;[1 1 1] Sphere_Find_04
      (if (== _sphere_find_04 (Variables|/Game/Blueprints/Player/Player_Ball_Bp.Player_Ball_Bp_C|GetClosest%20rail%20Sphere (stale EventTick _asplayer_ball_bp)))
        (Variables|Default|SetScene%20Component%20Object%20reference _sphere_find_04)))))

(event EventBeginPlay)

(event Collision|EventActorBeginOverlap
  (params (OtherActor :type Actor%20Object%20Reference)))

(event EventTick
  (params (DeltaSeconds :type Float%20%28single-precision%29))
  (bind _returnvalue (Utilities|Time|GetWorldDeltaSeconds))
  (bind _springarm (Variables|Default|GetSpringArm))
  (bind _springarm_2 (Variables|Default|GetSpringArm))
  ;[1 1 1] Remake
  (Utilities|FlowControl|Sequence
    (:then_0
      ;;[1 1 1] Comment
      (bind _asplayer_ball_bp (Utilities|Casting|CastToPlayer_Ball_Bp (Pawn|GetControlledPawn (Class|GameplayStatics|GetPlayerControllerfromID))))
      (Utilities|IsValid (Variables|/Game/Blueprints/Player/Player_Ball_Bp.Player_Ball_Bp_C|GetClosestSpline _asplayer_ball_bp)
        (:Is%20Valid
          (if (Variables|/Game/Blueprints/Player/Player_Ball_Bp.Player_Ball_Bp_C|GetVehicle%20has%20entered%20Rail%20sphere%20Trigger _asplayer_ball_bp)
            (CallFunction|AttatchPlayerCharactertotheRailSphere)
            (else
              (bind _output_get (Variables|Default|SetDistance%20of%20Cube%20along%20the%20spline (+ (Spline|GetDistanceAlongSplineatSplinePoint (Actor|GetComponentbyClass (Variables|/Game/Blueprints/Player/Player_Ball_Bp.Player_Ball_Bp_C|GetClosestSpline _asplayer_ball_bp) "/Script/Engine.SplineComponent") (Math|Float|Truncate (Class|SplineComponent|FindInputKeyClosesttoWorldLocation (Actor|GetComponentbyClass (Variables|/Game/Blueprints/Player/Player_Ball_Bp.Player_Ball_Bp_C|GetClosestSpline _asplayer_ball_bp) "/Script/Engine.SplineComponent") (Transformation|GetWorldLocation (Variables|Default|GetRail%20Actor))))) (* (- (Spline|GetDistanceAlongSplineatSplinePoint (Actor|GetComponentbyClass (Variables|/Game/Blueprints/Player/Player_Ball_Bp.Player_Ball_Bp_C|GetClosestSpline _asplayer_ball_bp) "/Script/Engine.SplineComponent") (Math|Float|Truncate (+ (Class|SplineComponent|FindInputKeyClosesttoWorldLocation (Actor|GetComponentbyClass (Variables|/Game/Blueprints/Player/Player_Ball_Bp.Player_Ball_Bp_C|GetClosestSpline _asplayer_ball_bp) "/Script/Engine.SplineComponent") (Transformation|GetWorldLocation (Variables|Default|GetRail%20Actor))) 1.0))) (Spline|GetDistanceAlongSplineatSplinePoint (Actor|GetComponentbyClass (Variables|/Game/Blueprints/Player/Player_Ball_Bp.Player_Ball_Bp_C|GetClosestSpline _asplayer_ball_bp) "/Script/Engine.SplineComponent") (Math|Float|Truncate (Class|SplineComponent|FindInputKeyClosesttoWorldLocation (Actor|GetComponentbyClass (Variables|/Game/Blueprints/Player/Player_Ball_Bp.Player_Ball_Bp_C|GetClosestSpline _asplayer_ball_bp) "/Script/Engine.SplineComponent") (Transformation|GetWorldLocation (Variables|Default|GetRail%20Actor)))))) (- (Math|Conversions|ToFloat(Integer) (Math|Float|Truncate (Class|SplineComponent|FindInputKeyClosesttoWorldLocation (Actor|GetComponentbyClass (Variables|/Game/Blueprints/Player/Player_Ball_Bp.Player_Ball_Bp_C|GetClosestSpline _asplayer_ball_bp) "/Script/Engine.SplineComponent") (Transformation|GetWorldLocation (Variables|Default|GetRail%20Actor))))) (Class|SplineComponent|FindInputKeyClosesttoWorldLocation (Actor|GetComponentbyClass (Variables|/Game/Blueprints/Player/Player_Ball_Bp.Player_Ball_Bp_C|GetClosestSpline _asplayer_ball_bp) "/Script/Engine.SplineComponent") (Transformation|GetWorldLocation (Variables|Default|GetRail%20Actor))))))))
              (Transformation|SetWorldLocationAndRotation (Variables|Default|GetRail%20Actor) (Spline|FindLocationClosesttoWorldLocation (Actor|GetComponentbyClass (Variables|/Game/Blueprints/Player/Player_Ball_Bp.Player_Ball_Bp_C|GetClosestSpline _asplayer_ball_bp) "/Script/Engine.SplineComponent") (Transformation|GetWorldLocation (Variables|/Game/Blueprints/Player/Player_Ball_Bp.Player_Ball_Bp_C|GetMovingSphere _asplayer_ball_bp)) "World") (Math|Rotator|MakeRotator (+ (.roll (Spline|GetRotationatDistanceAlongSpline (Actor|GetComponentbyClass (Variables|/Game/Blueprints/Player/Player_Ball_Bp.Player_Ball_Bp_C|GetClosestSpline _asplayer_ball_bp) "/Script/Engine.SplineComponent") _output_get "World")) (Variables|Default|GetRotational)) (.pitch (Spline|GetRotationatDistanceAlongSpline (Actor|GetComponentbyClass (Variables|/Game/Blueprints/Player/Player_Ball_Bp.Player_Ball_Bp_C|GetClosestSpline _asplayer_ball_bp) "/Script/Engine.SplineComponent") _output_get "World")) (.yaw (Spline|GetRotationatDistanceAlongSpline (Actor|GetComponentbyClass (Variables|/Game/Blueprints/Player/Player_Ball_Bp.Player_Ball_Bp_C|GetClosestSpline _asplayer_ball_bp) "/Script/Engine.SplineComponent") _output_get "World"))) false false)
              (Variables|Default|SetLast%20Known%20Rail%20Location _output_get)
              (Transformation|SetWorldLocationAndRotation (Variables|/Game/Blueprints/Player/Player_Ball_Bp.Player_Ball_Bp_C|GetCamera _asplayer_ball_bp) (Math|Interpolation|VInterpTo (Transformation|GetWorldLocation (Variables|/Game/Blueprints/Player/Player_Ball_Bp.Player_Ball_Bp_C|GetCamera _asplayer_ball_bp)) (Transformation|GetWorldLocation (Variables|/Game/Blueprints/Player/Player_Ball_Bp.Player_Ball_Bp_C|GetRemember%20Camera%20Location _asplayer_ball_bp)) 5.0 _returnvalue) (Math|Interpolation|RInterpTo (Transformation|GetWorldRotation (Variables|/Game/Blueprints/Player/Player_Ball_Bp.Player_Ball_Bp_C|GetCamera _asplayer_ball_bp)) (Transformation|GetWorldRotation (Variables|/Game/Blueprints/Player/Player_Ball_Bp.Player_Ball_Bp_C|GetRemember%20Camera%20Location _asplayer_ball_bp)) _returnvalue 5.0) false false))))))
    (:then_1
      ;[1 1 1] Turning
      (if (Variables|/Game/Blueprints/Player/Player_Ball_Bp.Player_Ball_Bp_C|GetVehicle%20has%20entered%20Rail%20sphere%20Trigger _asplayer_ball_bp)
        (Utilities|FlowControl|Sequence
          (:then_0
            (if (Game|Player|IsInputKeyDown (Game|GetPlayerController 0) "D")
              (bind _result (Math|Float|IncrementFloat (+ (Variables|Default|GetRotational) 5.0))
                (:%20%20
                  (Variables|Default|SetRotational _result)))))
          (:then_1
            (if (Game|Player|IsInputKeyDown (Game|GetPlayerController 0) "A")
              (bind _result_2 (Math|Float|DecrementFloat (- (Variables|Default|GetRotational) 5.0))
                (:%20%20
                  (Variables|Default|SetRotational _result_2))))))
        (else
          (Variables|Default|SetRotational 0.0))))
    (:then_2
      ;[1 1 1] Get Dot product
      (if (> (Math|Vector|DotProduct (Math|Vector|GetForwardVector (Variables|/Game/Blueprints/Player/Player_Ball_Bp.Player_Ball_Bp_C|GetFollowCube _asplayer_ball_bp)) (Transformation|GetActorForwardVector)) 0.0)
        (bind _output_get_2 (Variables|Default|SetFacing%20Right true))
        (else
          (bind _output_get_3 (Variables|Default|SetFacing%20Right false)))))
    (:then_3
      (if (Variables|Default|GetFacing%20Right)
        (Variables|Default|SetFacing%20Right%20Multiplier 1.0)
        (else
          (Variables|Default|SetFacing%20Right%20Multiplier -1.0))))
    (:then_4
      ;[1 1 1] Adjusting Camera Angle
      (if (Variables|Default|GetFacing%20Right)
        (Transformation|SetWorldRotation _springarm_2 (Math|Interpolation|RInterpTo (Transformation|GetWorldRotation _springarm_2) "-20.000000,0.000000, 0" (Utilities|Time|GetWorldDeltaSeconds) 3.0) false false)
        (else
          (Transformation|SetWorldRotation _springarm (Math|Interpolation|RInterpTo (Transformation|GetWorldRotation _springarm) "-20.000000,180.000000, 0" (Utilities|Time|GetWorldDeltaSeconds) 3.0) false false))))
    (:then_5
      (CallFunction|SettheFoundClosestRailSphere))
    (:then_6)))

(fn ConstructionScript)