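; Collectible coin that stays hidden until the player ball starts, then spins and awards score on pickup.
; Tick polls the trigger sphere's overlap with the ball instead of using overlap events, then raises mid-combo score and multiplier, refills the combo bar and flags controller shake.
; A delayed respawn at the saved transform follows DestroyActor, so it likely never fires.
; The game mode's DestroyCoins flag removes the coin.
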(event EventBeginPlay
  (Utilities|FlowControl|DoOnce false
    (:Completed
      (Rendering|SetVisibility (Variables|Default|GetSphere) false true)
      (Variables|Default|SetStarting%20Coin%20World%20Location (Transformation|GetWorldTransform (Variables|Default|GetSphereTrigger))))))

(event Collision|EventActorBeginOverlap
  (params (OtherActor :type Actor%20Object%20Reference)))

(event EventTick
  (params (DeltaSeconds :type Float%20%28single-precision%29))
  (bind _asplayer_ball_bp (Utilities|Casting|CastToPlayer_Ball_Bp (Game|Player|GetPlayerPawn 0)))
  (bind _asdefault_game_mode (Utilities|Casting|CastToDefaultGameMode (Game|GetGameMode)))
  (if (Variables|/Game/Levels_and_GameModes/DefaultGameMode.DefaultGameMode_C|GetDestroy%20coins _asdefault_game_mode)
    (Actor|DestroyActor)
    (elif (Variables|/Game/Blueprints/Player/Player_Ball_Bp.Player_Ball_Bp_C|GetStart _asplayer_ball_bp)
      (Rendering|SetVisibility (Variables|Default|GetSphere) true true)
      (Class|Actor|AddActorWorldRotation "0,3.000000, 0")
      (bind _asplayer_ball_bp_2 (Utilities|Casting|CastToPlayer_Ball_Bp (Game|Player|GetPlayerPawn 0)))
      (if (Class|PrimitiveComponent|IsOverlappingComponent (Variables|Default|GetSphereTrigger) (Variables|/Game/Blueprints/Player/Player_Ball_Bp.Player_Ball_Bp_C|GetMovingSphere _asplayer_ball_bp_2))
        (Actor|DestroyActor)
        (Variables|/Game/Blueprints/Player/Player_Ball_Bp.Player_Ball_Bp_C|SetMid%20Combo%20Player%20Score%20Var _asplayer_ball_bp_2 (+ (Variables|/Game/Blueprints/Player/Player_Ball_Bp.Player_Ball_Bp_C|GetMid%20Combo%20Player%20Score%20Var _asplayer_ball_bp_2) 10))
        (Variables|/Game/Blueprints/Player/Player_Ball_Bp.Player_Ball_Bp_C|SetActivate%20Coin%20Controller%20Shake _asplayer_ball_bp_2 true)
        (Variables|/Game/Blueprints/Player/Player_Ball_Bp.Player_Ball_Bp_C|SetActivate%20Combo%20Multiplier%20 _asplayer_ball_bp_2 true)
        (Variables|/Game/Blueprints/Player/Player_Ball_Bp.Player_Ball_Bp_C|SetCombo%20Bar%20Drain _asplayer_ball_bp_2 1e+02)
        (if (Variables|/Game/Blueprints/Player/Player_Ball_Bp.Player_Ball_Bp_C|GetActivate%20Combo%20Multiplier%20 _asplayer_ball_bp_2)
          (Variables|/Game/Blueprints/Player/Player_Ball_Bp.Player_Ball_Bp_C|SetCombo%20Mutliplier _asplayer_ball_bp_2 (+ (Variables|/Game/Blueprints/Player/Player_Ball_Bp.Player_Ball_Bp_C|GetCombo%20Mutliplier _asplayer_ball_bp_2) 1))
          (else
            (Variables|/Game/Blueprints/Player/Player_Ball_Bp.Player_Ball_Bp_C|SetCombo%20Mutliplier _asplayer_ball_bp_2 0)))
        (Utilities|FlowControl|Delay 5.0)
        (Game|SpawnActorfromClass "Coin_Collectible_C" (Variables|Default|GetStarting%20Coin%20World%20Location) "Undefined" 0 0)))))

(fn ConstructionScript)