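; Waypoint actor prop that creates a Challenge_Waypoint widget for the first player controller on BeginPlay.
; The graph neither stores the widget nor adds it to the viewport, and Tick is empty.
; Disconnected nodes hold an unused distance readout, which would convert the 2D distance to the Player_Ball_Bp's MovingSphere into text, truncated and divided by 100.
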(event EventBeginPlay
  (UserInterface|CreateWidget "/Game/User_Interface/Pointers/Challenge_Waypoint.Challenge_Waypoint_C" (Game|GetPlayerController 0)))

(event EventTick
  (params (DeltaSeconds :type Float%20%28single-precision%29)))

(fn ConstructionScript)