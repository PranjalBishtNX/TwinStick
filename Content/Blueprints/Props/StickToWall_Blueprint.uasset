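; StickToWall is a wall prop Blueprint that tracks the player ball and aims the ball's WallPointer at this wall's surface.
; Each Tick it casts player 0's pawn to Player_Ball_Bp and finds the closest collision point on its static mesh to the ball's MovingSphere.
; It sets the WallPointer's world rotation to look from the sphere toward that point, and draws a debug point there.
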(event EventBeginPlay)

(event Collision|EventActorBeginOverlap
  (params (OtherActor :type Actor%20Object%20Reference)))

(event EventTick
  (params (DeltaSeconds :type Float%20%28single-precision%29))
  (Utilities|FlowControl|Sequence
    (:then_0
      (bind _asplayer_ball_bp (Utilities|Casting|CastToPlayer_Ball_Bp (Pawn|GetControlledPawn (Class|GameplayStatics|GetPlayerControllerfromID))))
      (Transformation|SetWorldRotation (Variables|/Game/Blueprints/Player/Player_Ball_Bp.Player_Ball_Bp_C|GetWallPointer _asplayer_ball_bp) (Math|Rotator|FindLookatRotation (Transformation|GetWorldLocation (Variables|/Game/Blueprints/Player/Player_Ball_Bp.Player_Ball_Bp_C|GetMovingSphere _asplayer_ball_bp)) (.OutPointOnBody (Collision|GetClosestPointonCollision (Variables|Debug|GetStaticMeshComponent) (Transformation|GetWorldLocation (Variables|/Game/Blueprints/Player/Player_Ball_Bp.Player_Ball_Bp_C|GetMovingSphere _asplayer_ball_bp)) "None"))) false false)
      (Rendering|Debug|DrawDebugPoint (.OutPointOnBody (Collision|GetClosestPointonCollision (Variables|Debug|GetStaticMeshComponent) (Transformation|GetWorldLocation (Variables|/Game/Blueprints/Player/Player_Ball_Bp.Player_Ball_Bp_C|GetMovingSphere _asplayer_ball_bp)) "None")) 15.0 "(R=0.000000,G=0.000000,B=0.000000,A=1.000000)" 5.0))))

(fn ConstructionScript)