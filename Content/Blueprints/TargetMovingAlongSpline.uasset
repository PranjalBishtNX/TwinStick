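; Rail-ride actor that carries the player ball along a referenced spline through a follow cube.
; While the ball's rail attach flag is off, Tick snaps the cube to the spline point nearest the ball and derives its distance by interpolating the closest input key.
; While attached, it zeroes the ball's velocity, pins it to the cube and advances the cube a fixed distance per tick, making speed frame-rate dependent.
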(event EventBeginPlay)

(event Collision|EventActorBeginOverlap
  (params (OtherActor :type Actor%20Object%20Reference)))

(event EventTick
  (params (DeltaSeconds :type Float%20%28single-precision%29))
  (bind _spline_to_be_on (Variables|Default|GetSpline%20To%20Be%20on))
  (bind _followcubealongspline (Variables|Default|GetFollowCubeAlongSpline))
  (bind _returnvalue (Transformation|GetWorldLocation _followcubealongspline))
  (bind _spline (Variables|/Game/SplineActor.SplineActor_C|GetSpline _spline_to_be_on))
  (bind _returnvalue_2 (Class|SplineComponent|FindInputKeyClosesttoWorldLocation _spline _returnvalue))
  (bind _returnvalue_3 (Math|Float|Truncate _returnvalue_2))
  (bind _returnvalue_4 (Spline|GetDistanceAlongSplineatSplinePoint _spline _returnvalue_3))
  (bind _asplayer_ball_bp (Utilities|Casting|CastToPlayer_Ball_Bp (Pawn|GetControlledPawn (Class|GameplayStatics|GetPlayerControllerfromID))))
  (if (Variables|/Game/Blueprints/Player_Ball_Bp.Player_Ball_Bp_C|GetRail%20Attatch%20is%20active _asplayer_ball_bp)
    (Physics|SetPhysicsLinearVelocity (Variables|/Game/Blueprints/Player_Ball_Bp.Player_Ball_Bp_C|GetMovingShpere _asplayer_ball_bp) "0, 0, 0" false "None")
    (Transformation|SetWorldLocation (Variables|/Game/Blueprints/Player_Ball_Bp.Player_Ball_Bp_C|GetMovingShpere _asplayer_ball_bp) (Transformation|GetWorldLocation (Variables|Default|GetFollowCubeAlongSpline)) false false)
    (bind _output_get (Variables|Default|SetNewVar_0 (+ 2e+01 (Variables|Default|GetNewVar_0))))
    (Transformation|SetWorldLocation (Variables|Default|GetFollowCubeAlongSpline) (Spline|GetLocationatDistanceAlongSpline (Variables|/Game/SplineActor.SplineActor_C|GetSpline (Variables|Default|GetSpline%20To%20Be%20on)) _output_get "World") false false)
    (else
      (bind _output_get_2 (Variables|Default|SetDistance%20of%20Cube%20along%20the%20spline (+ _returnvalue_4 (* (- (Spline|GetDistanceAlongSplineatSplinePoint _spline (Math|Float|Truncate (+ _returnvalue_2 1.0))) _returnvalue_4) (- _returnvalue_2 (Math|Conversions|ToFloat(Integer) _returnvalue_3))))))
      (Transformation|SetWorldLocation (Variables|Default|GetFollowCubeAlongSpline) (Spline|FindLocationClosesttoWorldLocation (Variables|/Game/SplineActor.SplineActor_C|GetSpline (Variables|Default|GetSpline%20To%20Be%20on)) (Transformation|GetWorldLocation (Variables|/Game/Blueprints/Player_Ball_Bp.Player_Ball_Bp_C|GetMovingShpere _asplayer_ball_bp)) "World") false false)
      (Variables|Default|SetNewVar_0 _output_get_2))))

(fn ConstructionScript)