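; Game mode Blueprint for the Rolling game that runs a minutes-and-seconds countdown and flags coins for destruction when time expires.
; Tick checks for zero, then uses a one-second Delay while the timer runs to decrement seconds and roll over minutes.
; At zero it stops the timer and sets DestroyCoins.
; A ResetTimer event restores the starting time, but its DispatchResetTimer-gated trigger is unconnected and never runs.
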(event Custom|Reset%20Timer
  ;[1 1 1] Count Down timer
  (Variables|Default|SetMinutes 1)
  (Variables|Default|SetSeconds 30))

(event Custom|Check%20if%20countdown%20is%20over
  ;[1 1 1] Check if the countdown is over
  (if (<= (Variables|Default|GetMinutes) 0)
    (if (<= (Variables|Default|GetSeconds) 0)
      (Variables|Default|SetDestroy%20coins true)
      (Variables|Default|SetStart%20TImer false))))

(event EventTick
  (params (DeltaSeconds :type Float%20%28single-precision%29))
  ;[1 1 1] Count Down timer
  (CallFunction|CheckifCountdownIsOver)
  (if (Variables|Default|GetStart%20TImer)
    (Utilities|FlowControl|Delay 1.0)
    (Variables|Default|SetSeconds (- (Variables|Default|GetSeconds) 1))
    (if (< (Variables|Default|GetSeconds) 0)
      (Variables|Default|SetMinutes (- (Variables|Default|GetMinutes) 1))
      (Variables|Default|SetSeconds 59)
      (if true
        _))))

(fn ConstructionScript)